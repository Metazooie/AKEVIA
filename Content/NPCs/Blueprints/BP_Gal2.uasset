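; BP_Gal2 is an NPC animal actor that travels along the spline of a referenced track actor.
; On BeginPlay, if flagged active, it starts the WalkMover timeline at a configurable offset, with play rate scaled by Duration.
; Each update maps the timeline alpha to distance along the spline, setting the actor's world location and rotation from that point.
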(event `self.ReceiveBeginPlay`
  (if (`self.ActiveAnimal`)
    (`self.WalkAnimal`)))

(event `WalkAnimal`
  (bind _walkmover (`self.WalkMover`))
  (bind _returnvalue (`KismetMathLibrary.Lerp` 0.0 (`SplineComponent.GetSplineLength` (`/Game/NPCs/Blueprints/BP_Track.UsefulSpline` (`self.TrackRef`))) (`self.Alpha`)))
  (`TimelineComponent.SetPlayRate` _walkmover (/ 1.0 (`self.Duration`)))
  (`TimelineComponent.SetNewTime` _walkmover (`self.AnimalStartOffset`))
  (bind (_direction _alpha) (`Timeline|WalkMover`)
    (:`Update`
      (set `self.Alpha` _alpha)
      (`self.K2_SetActorLocationAndRotation` (`SplineComponent.GetLocationAtDistanceAlongSpline` (`/Game/NPCs/Blueprints/BP_Track.UsefulSpline` (`self.TrackRef`)) _returnvalue "World") (`SplineComponent.GetRotationAtDistanceAlongSpline` (`/Game/NPCs/Blueprints/BP_Track.UsefulSpline` (`self.TrackRef`)) _returnvalue "World")))))

(fn `UserConstructionScript`)