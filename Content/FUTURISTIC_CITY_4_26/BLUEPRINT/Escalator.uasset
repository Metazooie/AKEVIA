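; Animated escalator that endlessly moves a loop of steps up a slope using one InstancedStaticMesh.
; The construction script lays out the step instances, and a fast looping timer nudges each by a fixed increment.
; Near the top, steps flip 180 degrees with an offset and level out, then teleport back below the start.
; The separate ESCALATOR3 component is positioned half a step ahead of the transitioning step.
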(event `self.ReceiveBeginPlay`
  (`KismetSystemLibrary.K2_SetTimerDelegate` (delegate `timerEvent`) 0.01 true))

(event `timerEvent`
  (bind _returnvalue (* 16.0 63.0))
  (bind _instancedstaticmesh (`self.InstancedStaticMesh`))
  (bind _escalator_3 (`self.ESCALATOR_3`))
  (bind _returnvalue_2 (- (* 17.0 41.899689) (* 0.5 41.899689)))
  (for _index (range 20)
    (bind _y (.y (.location (`InstancedStaticMeshComponent.GetInstanceTransform` _instancedstaticmesh _index false))))
    (if (> _y (* 18.0 63.0))
      (`InstancedStaticMeshComponent.UpdateInstanceTransform` _instancedstaticmesh _index (`KismetMathLibrary.MakeTransform` (0.0 -63.0 -41.899689)) false true true)
      (elif (> _y (* 17.0 63.0))
        (bind _returnvalue_3 (+ (* 0.01 63.0 1.0) _y))
        (`InstancedStaticMeshComponent.UpdateInstanceTransform` _instancedstaticmesh _index (`KismetMathLibrary.MakeTransform` (`KismetMathLibrary.MakeVector` -147.0 _returnvalue_3 _returnvalue_2) (struct :`Yaw` 180.0)) false true true)
        (elif (> _y _returnvalue)
          (bind _returnvalue_4 (+ (* 0.01 41.899689 1.0) (.z (.location (`InstancedStaticMeshComponent.GetInstanceTransform` _instancedstaticmesh _index false)))))
          (bind _returnvalue_5 (- _returnvalue_4 (select `bool` (`KismetMathLibrary.NearlyEqual_FloatFloat` _y _returnvalue 0.01) :`true` (* 0.5 41.899689))))
          (`InstancedStaticMeshComponent.UpdateInstanceTransform` _instancedstaticmesh _index (`KismetMathLibrary.MakeTransform` (`KismetMathLibrary.MakeVector` -147.0 _returnvalue_3 _returnvalue_5) (struct :`Yaw` 180.0)) false true true)
          (bind _returnvalue_6 (+ _returnvalue_3 (* 0.5 63.0)))
          (if (< _returnvalue_6 (* 17.0 63.0))
            (`SceneComponent.K2_SetRelativeTransform` _escalator_3 (`KismetMathLibrary.MakeTransform` (`KismetMathLibrary.MakeVector` -147.0 _returnvalue_6 (+ _returnvalue_5 (* 0.5 41.899689))) (struct :`Yaw` 180.0)) false true)
            (`SceneComponent.SetVisibility` _escalator_3 true false)
            (else
              (`SceneComponent.K2_SetRelativeTransform` _escalator_3 (`KismetMathLibrary.MakeTransform` (`KismetMathLibrary.MakeVector` -147.0 (+ _returnvalue_3 (* 0.5 63.0)) _returnvalue_2) (struct :`Yaw` 180.0)) false true)
              (`SceneComponent.SetVisibility` _escalator_3 true false)))
          (else
            (`InstancedStaticMeshComponent.UpdateInstanceTransform` _instancedstaticmesh _index (`KismetMathLibrary.MakeTransform` (`KismetMathLibrary.MakeVector` (.x (.location (`InstancedStaticMeshComponent.GetInstanceTransform` _instancedstaticmesh _index false))) _returnvalue_3 _returnvalue_4)) false true true)))))))

(event `self.ReceiveTick`
  (params (DeltaSeconds :type "Float (single-precision)")))

(fn `UserConstructionScript`
  (for _index (range 20)
    (bind _returnvalue (* _index 63.0))
    (`InstancedStaticMeshComponent.AddInstance` (`self.InstancedStaticMesh`) (select `bool` (== _index 19) :`false` (`KismetMathLibrary.MakeTransform` (`KismetMathLibrary.MakeVector` 0.0 _returnvalue (* _index 41.899689))) :`true` (`KismetMathLibrary.MakeTransform` (`KismetMathLibrary.MakeVector` -147.0 _returnvalue (+ (* (- _index 1) 41.899689) (* 0.5 41.899689))) (struct :`Yaw` 180.0))))))