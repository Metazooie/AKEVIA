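; HUD Blueprint that runs a Photon Chat demo client and creates the main chat and settings widgets.
; On BeginPlay it caches the Photon chat and config references, binds chat events, adds the widgets and connects.
; Once connected it subscribes to channels, announces joins, feeds channel messages into the main widget and sends encrypted welcomes to newly seen users.
; Private-message display and on-screen connection-state drawing are disconnected.
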(event `self.ReceiveBeginPlay`
  (bind _playerowner (`self.PlayerOwner`))
  (bind _returnvalue (`PhotonCloudSubsystem.GetPhotonCloudAPI` (subsystem `PhotonCloudSubsystem`)))
  (`|ExecutionSequence`
    (:`then_0`
      ;[1 0.9015 0] Cache references
      (set `self.Photon Chat Ref` (`PhotonCloudObject.GetPhotonChat` _returnvalue))
      (set `self.Photon Config Ref` (`PhotonCloudObject.GetPhotonCloudConfig` _returnvalue)))
    (:`then_1`
      ;[1 0 0.6094] Bind events
      (add `PhotonChat.OnPhotonChatConnectionError` (`self.Photon Chat Ref`) (`|CreateDelegate` :!event `On Error Connecting`))
      (add `PhotonChat.OnPhotonChatSubscribeResults` (`self.Photon Chat Ref`) (`|CreateDelegate` :!event `On Photon Chat Subscribed`))
      (add `PhotonChat.OnPhotonChatGetMessages` (`self.Photon Chat Ref`) (`|CreateDelegate` :!event `On Photon Chat Received Messages`))
      (add `PhotonChat.OnPhotonChatStateChanged` (`self.Photon Chat Ref`) (`|CreateDelegate` :!event `On Chat State Updated`))
      (add `PhotonChat.OnPhotonChatGetPrivateMessage` (`self.Photon Chat Ref`) (`|CreateDelegate` :!event `On Photon Private Chat Message received`)))
    (:`then_2`
      ;[0 0.9766 1] Create Main Widget
      (bind _returnvalue_2 (`|CreateWidget` "/Game/PHOTON_MP/PHOTON_CHAT/ChatFeatures/Widgets/BP_ChatMainNewWidget.BP_ChatMainNewWidget_C" _playerowner))
      (bind _output_get (set `self.MainWidget` _returnvalue_2))
      (bind _returnvalue_3 (`|CreateWidget` "/Game/PHOTON_MP/PHOTON_CHAT/ChatFeatures/Widgets/BP_Settings.BP_Settings_C" _playerowner))
      (`UserWidget.AddToViewport` _output_get 0)
      (`UserWidget.AddToViewport` _returnvalue_3 0))
    (:`then_3`
      ;[0.5469 0 1] Everything ready: Connect!
      (`PhotonChat.Connect` (`self.Photon Chat Ref`)))))

(event `self.ReceiveDrawHUD`
  (params (SizeX :type Integer) (SizeY :type Integer))
  ;[0 0.625 1] Draws text to the Hud depending on whether its the Master client or a normal Client
)

(event `On Chat State Updated`
  (params (State :type "EChatConnectionState Enum" :default "NONE"))
  ;[1 0.5391 0] Subscribe on connect
  (`|ExecutionSequence`
    (:`then_1`
      (switch `EChatConnectionState` State
        (:`CONNECTED_CHAT`
          (`PhotonChat.SubscribeToChannels` (`self.Photon Chat Ref`) (`self.ChannelsToSubscribe`) 1))))))

(fn `On Error Connecting`
  (params (ErrorCode :type "EPhotonErrorCode Enum" :default "OK"))
  (`KismetSystemLibrary.PrintString` (`|GetEnumeratorNameAsString` ErrorCode) true true (struct :`R` 1.0 :`B` 0.38056 :`A` 1.0) 4.0))

(fn `On Photon Chat Received Messages`
  (params (ChannelName :type String) (Messages :type "Array of ChatMessage Structure (by ref)"))
  (for _array_element Messages
    (bind _returnvalue (`KismetStringLibrary.Concat_StrStr` (break `ChatMessage` _array_element) " : " (`.Message` (break `ChatMessage` _array_element))))
    (`KismetSystemLibrary.PrintString` _returnvalue)
    (`/Game/PHOTON_MP/PHOTON_CHAT/ChatFeatures/Widgets/BP_ChatMainNewWidget.Add Message Line` (`self.MainWidget`) _returnvalue))
  (if (and (not (`KismetArrayLibrary.Array_Contains` (`self.UserNames`) (break `ChatMessage` _array_element))) (`KismetStringLibrary.NotEqual_StrStr` (break `ChatMessage` _array_element) (`PhotonCloudConfig.chatUserID` (`self.Photon Config Ref`))))
    (`KismetArrayLibrary.Array_Add` (`self.UserNames`) (break `ChatMessage` _array_element))
    (`PhotonChat.SendPrivateMessage` (`self.Photon Chat Ref`) (break `ChatMessage` _array_element) (`KismetStringLibrary.Concat_StrStr` "Welcome, " (break `ChatMessage` _array_element) "!, nice to meet you!") true)))

(fn `On Photon Chat Subscribed`
  (params (ChannelsSubscribeResults :type "Array of ChatSubscribeResult Structure (by ref)"))
  (for _array_element ChannelsSubscribeResults
    (`KismetSystemLibrary.PrintString` (`KismetStringLibrary.Concat_StrStr` "Subscription to channel '" (break `ChatSubscribeResult` _array_element) (`KismetMathLibrary.SelectString` "  completed. Sending message to it" " not completed" (`.subscribed` (break `ChatSubscribeResult` _array_element)))))
    (bind _returnvalue (`KismetStringLibrary.Concat_StrStr` "Joined " (break `ChatSubscribeResult` _array_element)))
    (`/Game/PHOTON_MP/PHOTON_CHAT/ChatFeatures/Widgets/BP_ChatMainNewWidget.Add Message Line` (`self.MainWidget`) _returnvalue)
    (if (`.subscribed` (break `ChatSubscribeResult` _array_element))
      (`PhotonChat.SendMessage` (`self.Photon Chat Ref`) (break `ChatSubscribeResult` _array_element) _returnvalue)
      (set `/Game/PHOTON_MP/PHOTON_CHAT/ChatFeatures/Widgets/BP_ChatMainNewWidget.CurrentChannel` (break `ChatSubscribeResult` _array_element) (`self.MainWidget`)))))

(fn `On Photon Private Chat Message received`
  (params (UserName :type String) (ChannelName :type String) (Message :type String)))

(fn `UserConstructionScript`)